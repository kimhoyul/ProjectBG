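; Base Blueprint for items placed in the world, holding item identity, type, name, icon, capacity and mesh.
; On BeginPlay it line traces downward for Land-type objects and snaps itself to the hit location.
; Init functions fill the spawn and item data, and custom depth on the mesh toggles an outline.
; GetPickupData returns icon and name, with amount fixed at zero in this base.
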(event EventBeginPlay
  (bind _returnvalue (Transformation|GetActorLocation))
  ;[0.15 0.15 0.15 0.5] 아랫 방향으로 라인트레이스 를 쏴서 "오브젝트 타입"이 Land 인 녀석만 감지해서 해당 레이저가 맞은 위치로 지금 이 엑터의 좌표를 변경해주세요.
  (|CallParentFunction)
  (bind (_outhit _returnvalue_2) (Collision|LineTraceForObjects _returnvalue (+ _returnvalue (* (Math|Vector|VectorDown) 1e+03)) (Utilities|Array|MakeArray "ObjectTypeQuery7") false 0 "None"))
  (if _returnvalue_2
    (Transformation|SetActorLocation (.Location (Collision|BreakHitResult _outhit)) false false)))

(fn ConstructionScript
  (|CallParentFunction))

(fn InitSpwanData
  (params (ID :type Name) (SN :type String))
  (Variables|Default|SetID ID)
  (Variables|Default|SetSN SN))

(fn InitWroldItemBaseData
  (params (ItemType :type E_ItemType%20Enum :default "NewEnumerator0") (ItemName :type Text) (UIPrefix :type E_UIPrefix%20Enum :default "NewEnumerator0") (StaticMesh :type Static%20Mesh%20Object%20Reference) (ItemIcon :type Texture%202D%20Object%20Reference) (Capacity :type Integer))
  (Variables|Default|SetItemType ItemType)
  (Variables|Default|SetItemName ItemName)
  (Variables|Default|SetUIPrefix UIPrefix)
  (Components|StaticMesh|SetStaticMesh (Variables|Default|GetStaticMesh) StaticMesh)
  (Variables|Default|SetItem%20Icon ItemIcon)
  (Variables|Default|SetCapacity Capacity))

(fn EnableOutline
  (params (bIsEnabled :type Boolean))
  (Rendering|SetRenderCustomDepth (Variables|Default|GetStaticMesh) bIsEnabled))

(fn GetPickupData
  (return (Variables|Default|GetItem%20Icon) (Variables|Default|GetItemName) 0))