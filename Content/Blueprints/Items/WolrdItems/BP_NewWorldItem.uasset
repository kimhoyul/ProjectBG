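; World item actor that shows an item instance's mesh in the level and can be picked up or dropped.
; It assigns a GUID on BeginPlay if missing and takes its mesh from the item definition.
; Pickup routes by storage type to inventory or equipment, keeping any remainder or swapped-out item, otherwise destroying itself.
; Drops use an impulse with physics that switches off on sleep, and custom depth provides highlighting.
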(event OnComponentSleep(ItemMesh)
  (params (SleepingComponent :type Primitive%20Component%20Object%20Reference) (BoneName :type Name :default "None"))
  ;[0.15 0.15 0.15 0.5] 해당 루트 컴퍼넌트의 물리적 행동이 멈추면 실행
  (Physics|SetSimulatePhysics SleepingComponent false)
  (Collision|SetCollisionEnabled SleepingComponent "QueryOnly"))

(event EventBeginPlay
  ;[0.15 0.15 0.15 0.5] 아이템이 새로생성되면 ItemUID 가 비어있는데,  그 ID를 생성 (새로운 GUID)
  (if (not (Guid|IsValidGuid (Utilities|Struct|BreakST_NewItemInstance (Variables|Default|GetItemInstance))))
    (Utilities|Struct|SetmembersinST_NewItemInstance (Variables|Default|GetItemInstance) (Guid|NewGuid))
    (WroldItem|Visual|RefreshWorldItemVisual)))

(fn ConstructionScript
  (WroldItem|Visual|RefreshWorldItemVisual))

(fn RefreshWorldItemVisual
  (bind _iteminstance (Variables|Default|GetItemInstance))
  (bind _itemdefinition (Utilities|Struct|BreakST_NewItemInstance _iteminstance))
  (Utilities|IsValid _itemdefinition
    (:Is%20Valid
      (Components|StaticMesh|SetStaticMesh (Variables|Default|GetItemMesh) (Variables|/Game/Blueprints/Items/PDA_ItemDefinition.PDA_ItemDefinition_C|GetWorldMesh _itemdefinition)))))

(fn TryPickupItem
  (params (TargetInventoryRef :type BPC%20Inventory%20Object%20Reference) (TargetEquipmentRef :type BPC%20Equipment%20Object%20Reference) (TargetEquipmentSlot :type E_EquipmentSlot%20Enum :default "NewEnumerator0"))
  (Utilities|IsValid (Utilities|Struct|BreakST_NewItemInstance (Variables|Default|GetItemInstance))
    (:Is%20Valid
      (switch Utilities|FlowControl|Switch|SwitchonE_ItemStorageType (Variables|/Game/Blueprints/Items/PDA_ItemDefinition.PDA_ItemDefinition_C|GetStorageType (Utilities|Struct|BreakST_NewItemInstance (Variables|Default|GetItemInstance)))
        (:NewEnumerator0
          (return false 0 (Utilities|Struct|BreakST_NewItemInstance (Variables|Default|GetItemInstance))))
        (:NewEnumerator1
          (Utilities|IsValid TargetInventoryRef
            (:Is%20Valid
              (bind (_bsuccessed _addedquantity _remainingquantity) (Default|AddItem TargetInventoryRef (Variables|Default|GetItemInstance)))
              (if _bsuccessed
                (if (> _remainingquantity 0)
                  (Utilities|Struct|SetmembersinST_NewItemInstance (Variables|Default|GetItemInstance) _remainingquantity)
                  (WroldItem|Visual|RefreshWorldItemVisual)
                  (return true _addedquantity _remainingquantity)
                  (else
                    (Actor|DestroyActor)
                    (return true _addedquantity 0)))
                (else
                  (return _bsuccessed _addedquantity _remainingquantity))))
            (:Is%20Not%20Valid
              (return false 0 (Utilities|Struct|BreakST_NewItemInstance (Variables|Default|GetItemInstance))))))
        (:NewEnumerator2
          (Utilities|IsValid TargetEquipmentRef
            (:Is%20Valid
              (bind (_bsucceded _equippedslot _bhadreplaceditem _replaceditem) (Default|EquippedItem TargetEquipmentRef (Variables|Default|GetItemInstance) TargetEquipmentSlot))
              (if _bsucceded
                (if _bhadreplaceditem
                  (Variables|Default|SetItemInstance _replaceditem)
                  (WroldItem|Visual|RefreshWorldItemVisual)
                  (return true 1 (Utilities|Struct|BreakST_NewItemInstance _replaceditem))
                  (else
                    (Actor|DestroyActor)
                    (return true 1 0)))
                (else
                  (return false 0 (Utilities|Struct|BreakST_NewItemInstance (Variables|Default|GetItemInstance))))))
            (:Is%20Not%20Valid
              (return false 0 (Utilities|Struct|BreakST_NewItemInstance (Variables|Default|GetItemInstance))))))))
    (:Is%20Not%20Valid
      (return false 0 (Utilities|Struct|BreakST_NewItemInstance (Variables|Default|GetItemInstance))))))

(fn SetPickupHighlighted
  (params (bIsHighlighted :type Boolean))
  (Rendering|SetRenderCustomDepth (Variables|Default|GetItemMesh) bIsHighlighted))

(fn StartDropPhysics
  (params (DropDirection :type Vector))
  (Collision|SetCollisionEnabled (Variables|Default|GetItemMesh) "QueryAndPhysics")
  (Physics|SetSimulatePhysics (Variables|Default|GetItemMesh) true)
  (Physics|AddImpulse (Variables|Default|GetItemMesh) (+ (* DropDirection 1.2e+02) "0.000000,0.000000,60.000000") "None" false))