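; World item actor for a weapon accessory, such as a sight, muzzle, foregrip, magazine or buttstock.
; On spawn-data init it looks up its ID in DT_WorldItem_AccData, feeds the shared fields to the base item setup and stores accessory type and weight.
; It then applies the row's mesh rotation and offsets the actor along local Z by the mesh's bounds half-height, except for sights, which get no offset.
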(event EventBeginPlay
  (|CallParentFunction) ; This node is disabled and will not be called.\nDrag off pins to build functionality.
)

(event Collision|EventActorBeginOverlap
  (params (OtherActor :type Actor%20Object%20Reference)))

(event EventTick
  (params (DeltaSeconds :type Float%20%28single-precision%29)))

(fn ConstructionScript
  (|CallParentFunction))

(fn InitSpwanData
  (params (ID :type Name :default "None") (SN :type String))
  (bind _staticmesh (Variables|Default|GetStaticMesh))
  (bind _boxextent (Collision|GetComponentBounds _staticmesh))
  (|CallParentFunction ID SN)
  (bind _returnvalue (Utilities|GetDataTableRow "/Game/Blueprints/Datas/DataTable/Item/DT_WorldItem_AccData.DT_WorldItem_AccData" (Variables|Default|GetID))
    (:then
      (CallFunction|InitWroldItemBaseData (.itemtype _returnvalue) (.itemname _returnvalue) (.uiprefix _returnvalue) (.staticmesh _returnvalue) (.itemicon _returnvalue))
      (Variables|Default|SetAccType (.type _returnvalue))
      (Variables|Default|SetOut%20Row%20Weaight (.weaight _returnvalue))
      (Transformation|SetWorldRotation (Variables|Default|GetStaticMesh) (.rotationoffset _returnvalue) false false)
      (Transformation|AddActorLocalOffset (Math|Vector|MakeVector 0.0 0.0 (Utilities|Select :Index (Variables|Default|GetAccType) :NewEnumerator0 0.0 :NewEnumerator1 (.z _boxextent) :NewEnumerator2 (.z _boxextent) :NewEnumerator3 (.z _boxextent) :NewEnumerator4 (.z _boxextent))) false false))))