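; World item actor that represents an item instance in the level, showing its definition's mesh and assigning a GUID on BeginPlay if missing.
; TryPickupItem routes by storage type to an inventory or equipment component, leaving any remainder or swapped-out gear in place, otherwise destroying itself.
; Dropped items get an impulse with physics, which switches off to query-only collision once the mesh sleeps.
; Pickup highlighting toggles custom depth rendering.
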(event OnComponentSleep(ItemMesh)
  (params (SleepingComponent :type Primitive%20Component%20Object%20Reference) (BoneName :type Name :default "None"))
  (Physics|SetSimulatePhysics SleepingComponent false)
  (Collision|SetCollisionEnabled SleepingComponent "QueryOnly"))

(event EventBeginPlay
  (if (not (Guid|IsValidGuid (Utilities|Struct|BreakST_NewItemInstance (Variables|Default|GetItemInstance))))
    (bind _structout (Utilities|Struct|SetmembersinST_NewItemInstance (Variables|Default|GetItemInstance) (Guid|NewGuid)))
    (Variables|Default|SetItemInstance _structout)
    (WorldItem|Visual|RefreshWorldItemVisual)))

(fn ConstructionScript
  (WorldItem|Visual|RefreshWorldItemVisual))

(fn RefreshWorldItemVisual
  (bind _iteminstance (Variables|Default|GetItemInstance))
  (bind _itemdefinition (Utilities|Struct|BreakST_NewItemInstance _iteminstance))
  (Utilities|IsValid _itemdefinition
    (:Is%20Valid
      (Components|StaticMesh|SetStaticMesh (Variables|Components|GetItemMesh) (Variables|/Game/Blueprints/Items/BP_ItemDefinition.BP_ItemDefinition_C|GetWorldMesh _itemdefinition)))))

(fn TryPickupItem
  (params (TargetInventoryRef%20 :type BPC%20Inventory%20Object%20Reference) (TargetEquipmentRef :type BPC%20Equipment%20Object%20Reference))
  (Utilities|IsValid (Utilities|Struct|BreakST_NewItemInstance (Variables|Default|GetItemInstance))
    (:Is%20Valid
      (switch Utilities|FlowControl|Switch|SwitchonE_ItemStorageType (Variables|/Game/Blueprints/Items/BP_ItemDefinition.BP_ItemDefinition_C|GetStorageType (Utilities|Struct|BreakST_NewItemInstance (Variables|Default|GetItemInstance)))
        (:NewEnumerator0
          (return false 0 (Utilities|Struct|BreakST_NewItemInstance (Variables|Default|GetItemInstance))))
        (:NewEnumerator1
          (Utilities|IsValid TargetInventoryRef%20
            (:Is%20Valid
              (bind (_succeeded _addedquantity _remainingquantity) (Default|AddItem TargetInventoryRef%20 (Variables|Default|GetItemInstance)))
              (if _succeeded
                (if (> _remainingquantity 0)
                  (Utilities|Struct|SetmembersinST_NewItemInstance (Variables|Default|GetItemInstance) _remainingquantity)
                  (WorldItem|Visual|RefreshWorldItemVisual)
                  (return true _addedquantity _remainingquantity)
                  (else
                    (Actor|DestroyActor)
                    (return true _remainingquantity 0)))
                (else
                  (return _succeeded _addedquantity _remainingquantity))))
            (:Is%20Not%20Valid
              (return false 0 (Utilities|Struct|BreakST_NewItemInstance (Variables|Default|GetItemInstance))))))
        (:NewEnumerator2
          (Utilities|IsValid TargetEquipmentRef
            (:Is%20Valid
              (bind (_bsucceeded _equippedslot _bhadreplaceditem _replaceditem) (Default|EquipItem TargetEquipmentRef (Variables|Default|GetItemInstance)))
              (if _bsucceeded
                (if _bhadreplaceditem
                  (Variables|Default|SetItemInstance _replaceditem)
                  (WorldItem|Visual|RefreshWorldItemVisual)
                  (return true 1 (Utilities|Struct|BreakST_NewItemInstance _replaceditem))
                  (else
                    (Actor|DestroyActor)
                    (return true 1 0)))
                (else
                  (return false 0 (Utilities|Struct|BreakST_NewItemInstance (Variables|Default|GetItemInstance))))))
            (:Is%20Not%20Valid
              (return false 0 (Utilities|Struct|BreakST_NewItemInstance (Variables|Default|GetItemInstance))))))))
    (:Is%20Not%20Valid
      (return false 0 (Utilities|Struct|BreakST_NewItemInstance (Variables|Default|GetItemInstance))))))

(fn SetPickupHighlighted
  (params (bIsHighlighted :type Boolean))
  (Rendering|SetRenderCustomDepth (Variables|Components|GetItemMesh) bIsHighlighted))

(fn StartDropPhysics
  (params (DropDirection :type Vector))
  (Collision|SetCollisionEnabled (Variables|Components|GetItemMesh) "QueryAndPhysics")
  (Physics|SetSimulatePhysics (Variables|Components|GetItemMesh) true)
  (Physics|AddImpulse (Variables|Components|GetItemMesh) (+ (* DropDirection 1.2e+02) "0.000000,0.000000,60.000000") "None" true))