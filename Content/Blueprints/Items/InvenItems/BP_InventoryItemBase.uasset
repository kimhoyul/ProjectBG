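; BP_InventoryItemBase is a base Blueprint for inventory items, holding the shared data that describes an item.
; Its InventoryItemBaseData function takes ID, SN, item type, name, icon, capacity and amount and copies them into the matching variables.
; The event graph contains only disabled default events, and the construction script just calls its parent, so it has no other behavior.
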(event EventBeginPlay
  (|CallParentFunction) ; This node is disabled and will not be called.\nDrag off pins to build functionality.
)

(event Collision|EventActorBeginOverlap
  (params (OtherActor :type Actor%20Object%20Reference)))

(event EventTick
  (params (DeltaSeconds :type Float%20%28single-precision%29)))

(fn ConstructionScript
  (|CallParentFunction))

(fn InventoryItemBaseData
  (params (ID :type Name) (SN :type String) (ItemType :type E_ItemType%20Enum :default "NewEnumerator0") (ItemName :type Text) (ItemIcon :type Texture%202D%20Object%20Reference) (Capacity :type Integer) (Amount :type Integer))
  (Variables|Default|SetID ID)
  (Variables|Default|SetSN SN)
  (Variables|Default|SetItemType ItemType)
  (Variables|Default|SetItemName ItemName)
  (Variables|Default|SetItemIcon ItemIcon)
  (Variables|Default|SetCapacity Capacity)
  (Variables|Default|SetAmount Amount))