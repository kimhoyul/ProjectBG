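; BP_ItemGruop is an item group actor that generates random scattered positions around its own location.
; GetRandomTransforms returns the requested number of transforms, each offsetting the actor's location by a random direction scaled to a random distance.
; Only the X and Y of the random vectors are used, so points stay at the actor's height, with zero rotation and unit scale.
; The construction script is empty, and no spawning logic is present.
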(fn ConstructionScript)

(fn GetRandomTransforms
  (params (Number :type Integer))
  (bind _returnvalue (Math|Random|RandomFloatinRange 1e+02 2e+02))
  (bind _returnvalue_2 (Math|Random|RandomUnitVector))
  (bind _returnvalue_3 (* _returnvalue_2 _returnvalue))
  (for _index (range 1 Number)
    (Utilities|Array|Add (LocalVariables|GetReturnTransforms) (Math|Transform|MakeTransform (+ (Transformation|GetActorLocation) (Math|Vector|MakeVector (.x _returnvalue_3) (.y _returnvalue_3) 0.0)))))
  (return (LocalVariables|GetReturnTransforms)))