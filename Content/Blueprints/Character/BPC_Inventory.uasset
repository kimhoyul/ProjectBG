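; Character inventory component that stores item instances within a space-based capacity, the base value plus an equipment bonus.
; AddItem filters by storage type, accepts only what fits and merges stackables, issuing a new GUID when a partial pickup creates an entry.
; RemoveItem reduces or deletes entries by UID; both operations report quantities and fire OnInventoryChanged on success.
; A separate check tests whether a new equipment bonus still covers used space.
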(event EventBeginPlay)

(event EventTick
  (params (DeltaSeconds :type Float%20%28single-precision%29)))

(fn GetInventoryItems
  ;[0.15 0.15 0.15 0.5] 인벤토리 에 있는 아이템 배열 반환
  (return (Variables|Inventory|GetInventoryItems)))

(fn GetCurrentUsedSpace
  ;[0.15 0.15 0.15 0.5] 인벤토리가 사용하고 있는 전체 용량을 계산하는 함수
  (for _array_element (Variables|Inventory|GetInventoryItems)
    (Utilities|IsValid (.ItemDefinition (Utilities|Struct|BreakST_NewItemInstance _array_element))
      (:Is%20Valid
        (LocalVariables|SetTotalUserSpace (+ (LocalVariables|GetTotalUserSpace) (* (Variables|/Game/Blueprints/Items/PDA_ItemDefinition.PDA_ItemDefinition_C|GetSpacePerUnit (.ItemDefinition (Utilities|Struct|BreakST_NewItemInstance _array_element))) (.Quntity (Utilities|Struct|BreakST_NewItemInstance _array_element))))))))
  (return (LocalVariables|GetTotalUserSpace)))

(fn GetMaxCapacity
  ;[0.15 0.15 0.15 0.5] 최종 인벤토리 용량을 계산하는 함수
  (return (+ (Variables|Inventory|Capacity|GetBaseCapacity) (Variables|Inventory|Capacity|GetEquipmentCapacityBonus))))

(fn GetRemainingSpace
  ;[0.15 0.15 0.15 0.5] 현재 인벤토리에 남아 있는 용량 계산 함수
  (return (- (Inventory|Capacity|Query|GetMaxCapacity) (Inventory|Capacity|Query|GetCurrentUsedSpace))))

(fn CanStoreInventory
  (params (ItemDefinition :type PDA%20Item%20Definition%20Object%20Reference))
  ;[0.15 0.15 0.15 0.5] 전달받은 아이템이 가방 인벤토리에 들어갈 수 있는 아이템인지  하는 함수
  (Utilities|IsValid ItemDefinition
    (:Is%20Valid
      (return (and (Utilities|Enum|Equal(Enum) (Variables|/Game/Blueprints/Items/PDA_ItemDefinition.PDA_ItemDefinition_C|GetStorageType ItemDefinition) "NewEnumerator1") (> (Variables|/Game/Blueprints/Items/PDA_ItemDefinition.PDA_ItemDefinition_C|GetSpacePerUnit ItemDefinition) 0.0))))
    (:Is%20Not%20Valid
      (return false))))

(fn GetAddableQuantity
  (params (ItemDefinition :type PDA%20Item%20Definition%20Object%20Reference) (RequestQuantity :type Integer))
  ;[0.15 0.15 0.15 0.5] 요청받은 아이템 수량 중에서 현재 인벤토리에 실제로 몇 개 까지 들어갈 수 있는지 계산하는 함수
  (bind _bcanstore (Inventory|Query|CanStoreInventory ItemDefinition))
  (if _bcanstore
    (return (Math|Integer|Min(Integer) (Math|Integer|SelectInt RequestQuantity 0 (and (or (Variables|/Game/Blueprints/Items/PDA_ItemDefinition.PDA_ItemDefinition_C|GetStackable ItemDefinition) (== RequestQuantity 1)) (> RequestQuantity 0))) (Math|Float|Floor (/ (Inventory|Capacity|Query|GetRemainingSpace) (Variables|/Game/Blueprints/Items/PDA_ItemDefinition.PDA_ItemDefinition_C|GetSpacePerUnit ItemDefinition)))))
    (else
      (return 0))))

(fn FindMargeTargetIndex
  (params (ItemDefinition :type PDA%20Item%20Definition%20Object%20Reference))
  ;[0.15 0.15 0.15 0.5] 인벤토리 배열에서 새로 들어온 아이템과 수량을 합칠 수 있는 기존 항목의 인덱스를 찾는 함수
  (bind (_array_element _array_index) (Utilities|Array|ForEachLoopwithBreak (Variables|Inventory|GetInventoryItems) :!label _label)
    (:LoopBody
      (if (and (== (Utilities|Struct|BreakST_NewItemInstance _array_element) ItemDefinition) (Variables|/Game/Blueprints/Items/PDA_ItemDefinition.PDA_ItemDefinition_C|GetStackable ItemDefinition))
        (LocalVariables|SetResultIndex _array_index)
        (goto _label Break)))
    (:Completed
      (return (LocalVariables|GetResultIndex)))))

(fn AddorMargeInventoryItem
  (params (NewItem :type ST%20New%20Item%20Instance%20Structure) (QuantityToAdd :type Integer))
  ;[0.15 0.15 0.15 0.5] 인벤토리에 아이템을 추가하지만, 이미 배열에 있으면 수정, 없으면 생성
  (bind _foundindex (Inventory|Internal|FindMargeTargetIndex (Utilities|Struct|BreakST_NewItemInstance NewItem)))
  (bind _output_get (LocalVariables|SetMargeIndex _foundindex))
  (if (>= _output_get 0)
    (Utilities|Array|SetArrayElem (Variables|Inventory|GetInventoryItems) (LocalVariables|GetMargeIndex) (Utilities|Struct|MakeST_NewItemInstance (.ItemUID (Utilities|Struct|BreakST_NewItemInstance (Utilities|Array|Get(acopy) (Variables|Inventory|GetInventoryItems) (LocalVariables|GetMargeIndex)))) (.ItemDefinition (Utilities|Struct|BreakST_NewItemInstance (Utilities|Array|Get(acopy) (Variables|Inventory|GetInventoryItems) (LocalVariables|GetMargeIndex)))) (+ (.Quntity (Utilities|Struct|BreakST_NewItemInstance (Utilities|Array|Get(acopy) (Variables|Inventory|GetInventoryItems) (LocalVariables|GetMargeIndex)))) QuantityToAdd)))
    (else
      (Utilities|Array|Add (Variables|Inventory|GetInventoryItems) (Utilities|Struct|MakeST_NewItemInstance (select (== (.quntity NewItem) QuantityToAdd) (.itemuid NewItem) (Guid|NewGuid)) (.itemdefinition NewItem) QuantityToAdd)))))

(fn AddItem
  (params (NewItem :type ST%20New%20Item%20Instance%20Structure))
  (bind (_itemdefinition _quntity) (Utilities|Struct|BreakST_NewItemInstance NewItem))
  ;[0.15 0.15 0.15 0.5] 외부에서 호출할 실제 아이템 저장 함수
  (bind _addablequantity (Inventory|Query|GetAddableQuantity _itemdefinition _quntity))
  (bind _output_get (LocalVariables|SetQuantityToAdd _addablequantity))
  (if (> _output_get 0)
    (Inventory|Internal|AddorMargeInventoryItem NewItem (LocalVariables|GetQuantityToAdd))
    (Default|CallOnInventoryChanged)
    (return true (LocalVariables|GetQuantityToAdd) (- (Utilities|Struct|BreakST_NewItemInstance NewItem) (LocalVariables|GetQuantityToAdd)))
    (else
      (return false 0 (Math|Integer|Max(Integer) (Utilities|Struct|BreakST_NewItemInstance NewItem))))))

(fn FindItemIndexbyUID
  (params (ItemUID :type Guid%20Structure))
  ;[0.15 0.15 0.15 0.5] ItemUID 를 이용해서 인벤토리배열에서 특정 아이템을 찾아 인덱스 반환
  (if (Guid|IsValidGuid ItemUID)
    (bind (_array_element _array_index) (Utilities|Array|ForEachLoopwithBreak (Variables|Inventory|GetInventoryItems) :!label _label)
      (:LoopBody
        (if (== (Utilities|Struct|BreakST_NewItemInstance _array_element) ItemUID)
          (LocalVariables|SetResultIndex _array_index)
          (goto _label Break)))
      (:Completed
        (return (LocalVariables|GetResultIndex))))
    (else
      (return (LocalVariables|GetResultIndex)))))

(fn RemoveItem
  (params (ItemUID :type Guid%20Structure) (RequestQuntity :type Integer))
  ;[0.15 0.15 0.15 0.5] 외부에서 호출하는 인벤토리에서 특정 아이템을 실제로 제거하는 함수
  (bind _foundindex (Inventory|Internal|FindItemIndexbyUID ItemUID))
  (bind _output_get (LocalVariables|SetFoundIndex _foundindex))
  (if (and (>= _output_get 0) (> RequestQuntity 0))
    (Utilities|FlowControl|Sequence
      (:then_0
        ;;[0.15 0.15 0.15 0.5] 삭제할 아이템에 대한 전반적인 선 계산
        (LocalVariables|SetQuantityToRemove (Math|Integer|Min(Integer) (.Quntity (Utilities|Struct|BreakST_NewItemInstance (Utilities|Array|Get(acopy) (Variables|Inventory|GetInventoryItems) (LocalVariables|GetFoundIndex)))) RequestQuntity))
        (LocalVariables|SetLocalRemainingQuantity (- (.Quntity (Utilities|Struct|BreakST_NewItemInstance (Utilities|Array|Get(acopy) (Variables|Inventory|GetInventoryItems) (LocalVariables|GetFoundIndex)))) (LocalVariables|GetQuantityToRemove))))
      (:then_1
        (if (> (LocalVariables|GetLocalRemainingQuantity) 0)
          ;;[0.15 0.15 0.15 0.5] 인벤토리에 일부 아이템 남기기위해 수량만 수정
          (Utilities|Array|SetArrayElem (Variables|Inventory|GetInventoryItems) (LocalVariables|GetFoundIndex) (Utilities|Struct|MakeST_NewItemInstance (.ItemUID (Utilities|Struct|BreakST_NewItemInstance (Utilities|Array|Get(acopy) (Variables|Inventory|GetInventoryItems) (LocalVariables|GetFoundIndex)))) (.ItemDefinition (Utilities|Struct|BreakST_NewItemInstance (Utilities|Array|Get(acopy) (Variables|Inventory|GetInventoryItems) (LocalVariables|GetFoundIndex)))) (LocalVariables|GetLocalRemainingQuantity)))
          (else
            ;;[0.15 0.15 0.15 0.5] 인벤토리에서 전체 수량 삭제
            (Utilities|Array|RemoveIndex (Variables|Inventory|GetInventoryItems) (LocalVariables|GetFoundIndex)))))
      (:then_2
        (Default|CallOnInventoryChanged)
        (return true (LocalVariables|GetQuantityToRemove) (LocalVariables|GetLocalRemainingQuantity))))
    (else
      (return false 0 0))))

(fn SetEquipmentCapacityBonus
  (params (NewCapacityBonus :type Float%20%28double-precision%29))
  ;[0.15 0.15 0.15 0.5] 장비 장착시 가방 용량 추가, 감소 위한 함수
  (Variables|Inventory|Capacity|SetEquipmentCapacityBonus NewCapacityBonus))

(fn CanApplyEquipmentCapacity
  (params (NewEquipmentCapacityBonus :type Float%20%28double-precision%29))
  ;[0.15 0.15 0.15 0.5] 인벤토리 용량 기준으로 최대 용량변경을 할 수 있는지 검사하는 함수
  (return (<= (Inventory|Capacity|Query|GetCurrentUsedSpace) (+ NewEquipmentCapacityBonus (Variables|Inventory|Capacity|GetBaseCapacity)))))