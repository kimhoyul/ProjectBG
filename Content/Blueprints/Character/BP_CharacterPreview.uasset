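; Character preview actor that renders a copy of a player's body mesh into a supplied render target through a show-only scene capture.
; ApplyPlayerAppearance copies the player's skeletal mesh and loops an idle animation, currently always unarmed, with state-based selection left as a TODO.
; A pivot handles yaw rotation and reset.
; SetPreviewActive toggles mesh ticking and always stops per-frame capture, which StartPreviewCapture re-enables separately.
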(event EventBeginPlay)

(event Collision|EventActorBeginOverlap
  (params (OtherActor :type Actor%20Object%20Reference)))

(event EventTick
  (params (DeltaSeconds :type Float%20%28single-precision%29)))

(fn ConstructionScript)

(fn SetPreviewActive
  (params (bActive :type Boolean))
  (Variables|/Script/Engine.SceneCaptureComponent|SetbCaptureEveryFrame (Variables|Default|GetPreviewCapture) false)
  (Components|Tick|SetComponentTickEnabled (Variables|Default|GetBodyMesh) bActive))

(fn IsPreviewActive
  (return (Class|ActorComponent|IsComponentTickEnabled (Variables|Default|GetBodyMesh))))

(fn ResetPreviewRotation
  (Transformation|SetRelativeRotation (Variables|Default|GetPreviewPivot) "0.000000,180.000000,0.000000" false false))

(fn InitializeCapture
  (params (RenderTarget :type Texture%20Render%20Target%202D%20Object%20Reference))
  (bind _previewcapture (Variables|Default|GetPreviewCapture))
  (Variables|/Script/Engine.SceneCaptureComponent2D|SetTextureTarget _previewcapture RenderTarget)
  (Rendering|SceneCapture|ShowOnlyActorComponents _previewcapture self false))

(fn ApplyPlayerAppearance
  (params (SourcePlayer :type BP%20Player%20Object%20Reference))
  (bind _mesh (Variables|/Script/Engine.Character|GetMesh SourcePlayer))
  (bind _returnvalue (Components|SkeletalMesh|GetSkeletalMeshAsset _mesh))
  (Utilities|IsValid SourcePlayer
    (:Is%20Valid
      (Utilities|IsValid (Variables|/Script/Engine.Character|GetMesh SourcePlayer)
        (:Is%20Valid
          (if (!= (Components|SkeletalMesh|GetSkeletalMeshAsset (Variables|Default|GetBodyMesh)) _returnvalue)
            (Components|SkeletalMesh|SetSkeletalMeshAsset (Variables|Default|GetBodyMesh) _returnvalue)
            (Variables|Preview|Animation|SetCurrentPreviewIdle 0)
            (bind _bsuccss (Preview|Animation|ApplyPreviewIdle))
            (return _bsuccss)
            (else
              (Preview|Animation|ApplyPreviewIdle)
              (return true))))
        (:Is%20Not%20Valid
          _)))
    (:Is%20Not%20Valid
      _))
  (return false))

(fn ApplyPreviewIdle
  ;[0.15 0.15 0.15 0.5] TODO : 플레이어 상태(총을 들고있는지 근접 무기를 들던지 뭐든)에 따른 희망하는 애니메이션 선택 을 추가해야함
  (bind _output_get (LocalVariables|SetDesiredIdle (Variables|Preview|Animation|GetUnarmedIdeAnimation)))
  (Utilities|IsValid _output_get
    (:Is%20Valid
      (if (!= (LocalVariables|GetDesiredIdle) (Variables|Preview|Animation|GetCurrentPreviewIdle))
        (Components|Animation|PlayAnimation (Variables|Default|GetBodyMesh) (LocalVariables|GetDesiredIdle) true)
        (Variables|Preview|Animation|SetCurrentPreviewIdle (LocalVariables|GetDesiredIdle))
        (return true)
        (else
          (return true))))
    (:Is%20Not%20Valid
      (return false))))

(fn StartPreviewCapture
  (Variables|/Script/Engine.SceneCaptureComponent|SetbCaptureEveryFrame (Variables|Default|GetPreviewCapture) true))

(fn RotatePreview
  (params (DeltaYaw :type Float%20%28double-precision%29))
  (Transformation|AddLocalRotation (Variables|Default|GetPreviewPivot) (Math|Rotator|MakeRotator 0.0 0.0 (* DeltaYaw -1.0)) false false))