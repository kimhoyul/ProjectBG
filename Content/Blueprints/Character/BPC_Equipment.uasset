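; Actor component that tracks the owner's equipped items in a slot-keyed map and feeds their capacity bonuses to BPC_Inventory.
; Equip takes the slot from PDA_EquipmentDefinition and returns any replaced item; equip and unequip both fail unless the inventory accepts the projected bonus total.
; Successful changes push the recomputed bonus and fire an equipment-changed notification.
; A helper matches a weapon UID against one fixed slot.
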(event EventBeginPlay
  (Variables|Equipment|References|SetInventoryComponentRef (Actor|GetComponentbyClass (Components|GetOwner) "/Game/Blueprints/Character/BPC_Inventory.BPC_Inventory_C"))
  (Equipment|Capacity|Internal|RefreshInventoryCapacityBonus))

(fn GetEquippedItem
  (params (Slot :type E_EquipmentSlot%20Enum :default "NewEnumerator0"))
  (bind _equippeditems (Variables|Equipment|Data|GetEquippedItems))
  (bind (_value _returnvalue) (Utilities|Map|Find _equippeditems Slot))
  (return _value _returnvalue))

(fn IsSlotOccupied
  (params (Slot :type E_EquipmentSlot%20Enum :default "NewEnumerator0"))
  (return (Utilities|Map|Contains (Variables|Equipment|Data|GetEquippedItems) Slot)))

(fn SetEquippedItem
  (params (Slot :type E_EquipmentSlot%20Enum :default "NewEnumerator0") (Item :type ST%20New%20Item%20Instance%20Structure))
  (Utilities|Map|Add (Variables|Equipment|Data|GetEquippedItems) Slot Item)
  (Equipment|Capacity|Internal|RefreshInventoryCapacityBonus)
  (Default|CallOnEquipmentChanged Slot Item))

(fn EquipItem
  (params (NewItem :type ST%20New%20Item%20Instance%20Structure))
  (bind _aspda_equipment_definition (Utilities|Casting|CastToPDA_EquipmentDefinition (Utilities|Struct|BreakST_NewItemInstance NewItem))
    (:then
      (bind _output_get (LocalVariables|SetTargetSlot (Variables|/Game/Blueprints/Items/PDA_EquipmentDefinition.PDA_EquipmentDefinition_C|GetEquipmentSlot _aspda_equipment_definition)))
      (LocalVariables|SetPreviousItem (.Item (Equipment|Query|GetEquippedItem _output_get)))
      (LocalVariables|SetbHadPreviousItem (.bFound (Equipment|Query|GetEquippedItem _output_get)))
      (bind _output_get_2 (LocalVariables|SetCurrentTotalCapacityBonus (Equipment|Capacity|Query|GetTotalCapacityBonus)))
      (Utilities|IsValid (Variables|Equipment|References|GetInventoryComponentRef)
        (:Is%20Valid
          (if (Default|CanApplyEquipmentCapacityBonus (Variables|Equipment|References|GetInventoryComponentRef) (+ (- _output_get_2 (Equipment|Capacity|Query|GetItemCapacityBonus (LocalVariables|GetPreviousItem))) (Equipment|Capacity|Query|GetItemCapacityBonus NewItem)))
            (Equipment|Internal|SetEquippedItem (LocalVariables|GetTargetSlot) NewItem)
            (return true (LocalVariables|GetTargetSlot) (LocalVariables|GetbHadPreviousItem) (LocalVariables|GetPreviousItem))
            (else
              _)))
        (:Is%20Not%20Valid
          _))
      (return false (LocalVariables|GetTargetSlot) false ""))
    (:CastFailed
      (return false "NewEnumerator0" false ""))))

(fn UnequipItem
  (params (Slot :type E_EquipmentSlot%20Enum :default "NewEnumerator0"))
  (bind _equippeditems (Variables|Equipment|Data|GetEquippedItems))
  (bind (_value _returnvalue) (Utilities|Map|Find _equippeditems Slot))
  (if _returnvalue
    (LocalVariables|SetItemToUnequip _value)
    (Utilities|IsValid (Variables|Equipment|References|GetInventoryComponentRef)
      (:Is%20Valid
        (if (Default|CanApplyEquipmentCapacityBonus (Variables|Equipment|References|GetInventoryComponentRef) (- (Equipment|Capacity|Query|GetTotalCapacityBonus) (Equipment|Capacity|Query|GetItemCapacityBonus (LocalVariables|GetItemToUnequip))))
          (Utilities|Map|Remove (Variables|Equipment|Data|GetEquippedItems) Slot)
          (Equipment|Capacity|Internal|RefreshInventoryCapacityBonus)
          (Default|CallOnEquipmentChanged Slot)
          (return true (LocalVariables|GetItemToUnequip))
          (else
            (return false ""))))
      (:Is%20Not%20Valid
        (return false "")))
    (else
      (return false ""))))

(fn GetItemCapacityBonus
  (params (Item :type ST%20New%20Item%20Instance%20Structure))
  (bind _aspda_equipment_definition (Utilities|Casting|CastToPDA_EquipmentDefinition (Utilities|Struct|BreakST_NewItemInstance Item))
    (:then
      (return (Variables|/Game/Blueprints/Items/PDA_EquipmentDefinition.PDA_EquipmentDefinition_C|GetCapacityBonus _aspda_equipment_definition)))
    (:CastFailed
      (return 0.0))))

(fn GetTotalCapacityBonus
  (bind _values (Utilities|Map|Values (Variables|Equipment|Data|GetEquippedItems)))
  (for _array_element _values
    (LocalVariables|SetCalculatedCapacityBonus (+ (Equipment|Capacity|Query|GetItemCapacityBonus _array_element) (LocalVariables|GetCalculatedCapacityBonus))))
  (return (LocalVariables|GetCalculatedCapacityBonus)))

(fn RefreshInventoryCapacityBonus
  (bind _inventorycomponentref (Variables|Equipment|References|GetInventoryComponentRef))
  (Utilities|IsValid _inventorycomponentref
    (:Is%20Valid
      (Default|SetEquipmentCapacityBonus _inventorycomponentref (Equipment|Capacity|Query|GetTotalCapacityBonus)))))

(fn FindPrimaryWeaponSlotbyUID
  (params (WeaponUID :type Guid%20Structure))
  (bind (_item _bfound) (Equipment|Query|GetEquippedItem "NewEnumerator4"))
  (if (and (== WeaponUID (Utilities|Struct|BreakST_NewItemInstance _item)) _bfound)
    (return true "NewEnumerator4")))