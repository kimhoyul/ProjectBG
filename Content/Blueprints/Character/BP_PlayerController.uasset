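; Player controller for BP_Player that handles look, free look, jump, crouch/prone, walk/run input and switches UI input mode.
; Pose changes resolve target pose and transition time from DataTables, clearing a move-enable flag during timed transitions.
; Each pose loads DataTable pitch limits and camera height, with timelines easing out-of-range pitch and spring-arm offset.
; Crouch camera height also varies with movement and weapon state.
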(event Custom|OnMovementStateChanged
  (params (bIsMoving :type Boolean))
  (Camera|UpdateCameraHeight bIsMoving))

(event Custom|SetEnableMove
  ;[0.15 0.15 0.15 0.5] 포즈변경
  (Variables|Move|SetbIsEnableMove true))

(event Input|EnhancedActionEvents|EnhancedInputActionIA_Look
  (params (ActionValue :type Vector%202D%20Structure) (ElapsedSeconds :type Float%20%28double-precision%29) (TriggeredSeconds :type Float%20%28double-precision%29) (InputAction :type Input%20Action%20Object%20Reference :default "/Game/Input/Actions/IA_Look.IA_Look"))
  (bind (_x _y) (Math|Vector2D|BreakVector2D ActionValue))
  ;[0.15 0.15 0.15 0.5] 카메라회전
  (if (not (Variables|Default|GetbShowMouseCursor))
    (Utilities|FlowControl|Sequence
      (:then_0
        (Default|InputTurn (Variables|Ref|GetPlayerRef) _x))
      (:then_1
        (if (Camera|LimitPitchAngle _y)
          (Default|InputLookUp (Variables|Ref|GetPlayerRef) _y)))
      (:then_2
        (Default|UpdateTargetingItem (Variables|Ref|GetPlayerRef))))))

(event EventBeginPlay
  (bind _playerref (Variables|Ref|GetPlayerRef))
  ;[0.15 0.15 0.15 0.5] 참조 캐싱
  (Initializ|InitializeReferences)
  ;[0.15 0.15 0.15 0.5] 카메라 각도 제한 초기화
  (Camera|UpdatePitchLimits "NewEnumerator0")
  (EventDispatchers|BindEventtoOnMovementStateChanged _playerref (delegate Custom|OnMovementStateChanged))
  (Default|CachedWalkSpeedbyPose _playerref)
  (Input|AddMappingContext (PlayerController|LocalPlayerSubsystems|GetEnhancedInputLocalPlayerSubsystem) "/Game/Input/IMC_Default.IMC_Default" 0 "(bIgnoreAllPressedKeysUntilRelease=True,bForceImmediately=False,bNotifyUserSettings=False)"))

(event Input|ActionEvents|InputActionFreeLook
  (params (Key :type Key%20Structure))
  (bind _playerref (Variables|Ref|GetPlayerRef))
  ;[0.15 0.15 0.15 0.5] 자유시점
  (:Pressed
    (Default|FreeLook _playerref true))
  (:Released
    (Default|FreeLook _playerref false)))

(event Input|ActionEvents|InputActionProne
  (params (Key :type Key%20Structure))
  (bind _playerref (Variables|Ref|GetPlayerRef))
  (bind _bisweaponequipped (Variables|/Game/Blueprints/Character/BP_Player.BP_Player_C|GetbIsWeaponEquipped _playerref))
  (bind _currentposestate (Variables|/Game/Blueprints/Character/BP_Player.BP_Player_C|GetCurrentPoseState _playerref))
  (bind (_transitiontime _topose) (Pose|OnTransitionTimer _bisweaponequipped "NewEnumerator2" _currentposestate))
  ;[0.15 0.15 0.15 0.5] 포즈변경
  (:Pressed
    (Pose|UpdatePose _transitiontime _topose)))

(event Input|ActionEvents|InputActionJump
  (params (Key :type Key%20Structure))
  (bind _playerref (Variables|Ref|GetPlayerRef))
  (bind _currentposestate (Variables|/Game/Blueprints/Character/BP_Player.BP_Player_C|GetCurrentPoseState _playerref))
  (bind _bisweaponequipped (Variables|/Game/Blueprints/Character/BP_Player.BP_Player_C|GetbIsWeaponEquipped _playerref))
  (bind (_transitiontime _topose) (Pose|OnTransitionTimer _bisweaponequipped "NewEnumerator0" _currentposestate))
  ;[0.15 0.15 0.15 0.5] 포즈변경
  (:Pressed
    (if (Utilities|Enum|Equal(Enum) _currentposestate "NewEnumerator0")
      (Character|Jump (Variables|Ref|GetPlayerRef))
      (else
        (Pose|UpdatePose _transitiontime _topose)))))

(event Input|ActionEvents|InputActionWalk
  (params (Key :type Key%20Structure))
  (bind _playerref (Variables|Ref|GetPlayerRef))
  ;[0.15 0.15 0.15 0.5] Walk : 누르면 상태가 Walk, 안누르면 Jog
  (:Pressed
    (Variables|/Game/Blueprints/Character/BP_Player.BP_Player_C|SetbIsWalkPressed _playerref true)
    (Default|EvaluateMoveState _playerref :!label _label)
    (Default|CachedWalkSpeedbyPose _playerref))
  (:Released
    (Variables|/Game/Blueprints/Character/BP_Player.BP_Player_C|SetbIsWalkPressed _playerref false)
    (goto _label)))

(event Input|ActionEvents|InputActionRun
  (params (Key :type Key%20Structure))
  (bind _playerref (Variables|Ref|GetPlayerRef))
  ;[0.15 0.15 0.15 0.5] Run : 누르면 상태가 Run, 안누르면 Jog
  (:Pressed
    (Variables|/Game/Blueprints/Character/BP_Player.BP_Player_C|SetbIsRunPressed _playerref true)
    (Default|EvaluateMoveState _playerref :!label _label)
    (Default|CachedWalkSpeedbyPose _playerref))
  (:Released
    (Variables|/Game/Blueprints/Character/BP_Player.BP_Player_C|SetbIsRunPressed _playerref false)
    (goto _label)))

(event Input|ActionEvents|InputActionCrouch
  (params (Key :type Key%20Structure))
  (bind _playerref (Variables|Ref|GetPlayerRef))
  (bind _currentposestate (Variables|/Game/Blueprints/Character/BP_Player.BP_Player_C|GetCurrentPoseState _playerref))
  (bind _bisweaponequipped (Variables|/Game/Blueprints/Character/BP_Player.BP_Player_C|GetbIsWeaponEquipped _playerref))
  (bind (_transitiontime _topose) (Pose|OnTransitionTimer _bisweaponequipped "NewEnumerator1" _currentposestate))
  ;[0.15 0.15 0.15 0.5] 포즈변경
  (:Pressed
    (Pose|UpdatePose _transitiontime _topose)))

(event Custom|ChangePitchLimit
  (params (CurrentRotator :type Rotator) (TargetRotator :type Rotator))
  (bind _alpha (Timeline|Timeline PlayFromStart)
    (:Update
      (Pawn|SetControlRotation (Math|Rotator|Lerp(Rotator) CurrentRotator TargetRotator _alpha true)))))

(event Custom|ChangeCameraHeight
  (params (StartHeigtht :type Vector) (TargetHeight :type Vector))
  (bind _alpha (Timeline|Timeline_0 PlayFromStart)
    (:Update
      (Variables|/Script/Engine.SpringArmComponent|SetSocketOffset (Variables|/Game/Blueprints/Character/BP_Player.BP_Player_C|GetSpringArm (Variables|Ref|GetPlayerRef)) (Math|Vector|Lerp(Vector) StartHeigtht TargetHeight _alpha)))))

(fn ConstructionScript)

(fn TryGetPoseTransition
  (params (TargetPose :type E_PoseState%20Enum :default "NewEnumerator0") (FromPose :type E_PoseState%20Enum :default "NewEnumerator0"))
  (bind _returnvalue (Utilities|GetDataTableRow "/Game/Blueprints/Datas/DataTable/Character/DT_PoseTransitionRule.DT_PoseTransitionRule" (Utilities|String|StringToName (Utilities|String|Append (Utilities|String|EnumtoString TargetPose) "_" (Utilities|String|EnumtoString FromPose))))
    (:then
      (return (.topose _returnvalue)))))

(fn OnTransitionTimer
  (params (bIsWeaponEquipped :type Boolean) (TargetPose :type E_PoseState%20Enum :default "NewEnumerator0") (FromPose :type E_PoseState%20Enum :default "NewEnumerator0"))
  (LocalVariables|SetReturnPose (Pose|TryGetPoseTransition TargetPose FromPose))
  (bind _returnvalue (Utilities|GetDataTableRow "/Game/Blueprints/Datas/DataTable/Character/DT_ProneTime.DT_ProneTime" (Utilities|String|StringToName (Utilities|String|Append (Utilities|String|ToString(Boolean) bIsWeaponEquipped) "_" (Utilities|String|EnumtoString FromPose) "_" (Utilities|String|EnumtoString (LocalVariables|GetReturnPose)))))
    (:then
      _)
    (:RowNotFound
      _))
  (return (.sec _returnvalue) (LocalVariables|GetReturnPose)))

(fn UpdatePose
  (params (WaitTime :type Float%20%28double-precision%29) (ToPose :type E_PoseState%20Enum :default "NewEnumerator0"))
  (Utilities|FlowControl|Sequence
    (:then_0
      (if (!= WaitTime 0.0)
        (Variables|Move|SetbIsEnableMove false)
        (Utilities|Time|SetTimerbyEvent (EventDispatchers|CreateEvent :!event Custom|SetEnableMove) WaitTime)
        (Default|UpdatePoseState (Variables|Ref|GetPlayerRef) ToPose)
        (else
          (Default|UpdatePoseState (Variables|Ref|GetPlayerRef) ToPose))))
    (:then_1
      (Camera|UpdatePitchLimits ToPose)
      (Camera|UpdateCameraHeight (Variables|/Game/Blueprints/Character/BP_Player.BP_Player_C|GetbIsMovingNow (Variables|Ref|GetPlayerRef)))
      (Default|CachedWalkSpeedbyPose (Variables|Ref|GetPlayerRef)))))

(fn UpdatePitchLimits
  (params (NewState :type E_PoseState%20Enum :default "NewEnumerator0"))
  (bind _returnvalue (Pawn|GetControlRotation :!class /Script/Engine.Controller))
  (Utilities|FlowControl|Sequence
    (:then_0
      (bind _returnvalue_2 (Utilities|GetDataTableRow "/Game/Blueprints/Datas/DataTable/Character/DT_PitchLimit.DT_PitchLimit" (Utilities|String|StringToName (Utilities|String|EnumtoString NewState)))
        (:then
          (Variables|Camera|SetCachedTopLimit (.toplimit _returnvalue_2))
          (Variables|Camera|SetCachedBottomLimit (.bottomlimit _returnvalue_2)))))
    (:then_1
      ;[0.15 0.15 0.15 0.5] 현재 카메라 각도가 리밋 각도를 초과했는지 확인
      (if (not (or (> (.pitch _returnvalue) (Variables|Camera|GetCachedBottomLimit)) (< (.pitch _returnvalue) (Variables|Camera|GetCachedTopLimit))))
        ;[0.15 0.15 0.15 0.5] 무조건 리밋값으로 카메라를 강제 회전
        (if (< (Math|Float|Absolute(Float) (- (.pitch _returnvalue) (Variables|Camera|GetCachedTopLimit))) (Math|Float|Absolute(Float) (- (.pitch _returnvalue) (Variables|Camera|GetCachedBottomLimit))))
          (CallFunction|ChangePitchLimit (.CurrentRotator (Camera|MakeViewRotator (Variables|Camera|GetCachedTopLimit))) (.TargetRotator (Camera|MakeViewRotator (Variables|Camera|GetCachedTopLimit))))
          (else
            (CallFunction|ChangePitchLimit (.CurrentRotator (Camera|MakeViewRotator (Variables|Camera|GetCachedBottomLimit))) (.TargetRotator (Camera|MakeViewRotator (Variables|Camera|GetCachedBottomLimit))))))))))

(fn LimitPitchAngle
  (params (Axis :type Float%20%28double-precision%29))
  (bind _returnvalue (Class|PlayerController|GetDeprecatedInputPitchScale))
  (bind _returnvalue_2 (Pawn|GetControlRotation :!class /Script/Engine.Controller))
  (bind _returnvalue_3 (* Axis _returnvalue))
  (bind _returnvalue_4 (+ (.pitch _returnvalue_2) _returnvalue_3))
  (return (or (> _returnvalue_4 (Variables|Camera|GetCachedBottomLimit)) (< _returnvalue_4 (Variables|Camera|GetCachedTopLimit)))))

(fn MakeViewRotator
  (params (LimitPitch :type Float%20%28double-precision%29))
  (bind _returnvalue (Pawn|GetControlRotation :!class /Script/Engine.Controller))
  (bind (_roll _pitch _yaw) (Math|Rotator|BreakRotator _returnvalue))
  (return _returnvalue (Math|Rotator|MakeRotator _roll LimitPitch _yaw)))

(fn UpdateCameraHeight
  (params (bIsMovingNow :type Boolean))
  (bind _playerref (Variables|Ref|GetPlayerRef))
  (bind _playerref_2 (Variables|Ref|GetPlayerRef))
  (bind _currentposestate (Variables|/Game/Blueprints/Character/BP_Player.BP_Player_C|GetCurrentPoseState _playerref))
  (bind _springarm (Variables|/Game/Blueprints/Character/BP_Player.BP_Player_C|GetSpringArm _playerref_2))
  (bind _socketoffset (Variables|/Script/Engine.SpringArmComponent|GetSocketOffset _springarm))
  (Utilities|FlowControl|Sequence
    (:then_0
      (LocalVariables|SetCurrentPose (Utilities|String|EnumtoString _currentposestate))
      (if (Utilities|Enum|NotEqual(Enum) _currentposestate "NewEnumerator1")
        ;[0.15 0.15 0.15 0.5] Crouch 아니라면 현재상태가 곧 RowName
        (LocalVariables|SetRowName (LocalVariables|GetCurrentPose))
        (else
          (LocalVariables|SetRowName (LocalVariables|GetCurrentPose))
          (if bIsMovingNow
            (LocalVariables|SetRowName (Utilities|String|Append (LocalVariables|GetRowName) "_" (Utilities|String|ToString(Boolean) (Variables|/Game/Blueprints/Character/BP_Player.BP_Player_C|GetbIsWeaponEquipped (Variables|Ref|GetPlayerRef))) "_Move"))))))
    (:then_1
      (bind _returnvalue (Utilities|GetDataTableRow "/Game/Blueprints/Datas/DataTable/Character/DT_CameraHeight.DT_CameraHeight" (Utilities|String|StringToName (LocalVariables|GetRowName)))
        (:then
          (CallFunction|ChangeCameraHeight (Variables|/Script/Engine.SpringArmComponent|GetSocketOffset (Variables|/Game/Blueprints/Character/BP_Player.BP_Player_C|GetSpringArm (Variables|Ref|GetPlayerRef))) (Math|Vector|MakeVector (.x _socketoffset) (.y _socketoffset) (.height _returnvalue))))))))

(fn RequestUI
  (params (UIType :type E_UIType%20Enum :default "NewEnumerator0"))
  (bind _hudref (Variables|Ref|GetHUDRef))
  (Utilities|IsValid _hudref
    (:Is%20Valid
      (Default|ProcessUIReqeust _hudref UIType))))

(fn InitializeReferences
  (bind _asbp_player (Utilities|Casting|CastToBP_Player (Game|GetPlayerCharacter 0)))
  (Variables|Ref|SetPlayerRef _asbp_player)
  (bind _asbp_hud (Utilities|Casting|CastToBP_HUD (HUD|GetHUD)))
  (Variables|Ref|SetHUDRef _asbp_hud))

(fn ApplyUIInputMode
  (params (bIsUIOpen :type Boolean))
  (if bIsUIOpen
    (Input|SetInputModeGameandUI self 0 "DoNotLock" false false)
    (Variables|Default|SetbShowMouseCursor true)
    (else
      (Input|SetInputModeGameOnly self false)
      (Variables|Default|SetbShowMouseCursor false))))